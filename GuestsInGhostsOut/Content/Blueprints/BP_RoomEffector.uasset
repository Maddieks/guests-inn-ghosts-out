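; BP_RoomEffector is a short-lived actor that exposes heat, locomotive disturbance and noisiness values, apparently as a temporary influence on a room.
; It accumulates Age on Tick and destroys itself once a Delay of Lifespan seconds elapses after BeginPlay.
; Its getters scale each base value by Age over Lifespan, guarded against zero, so every effect ramps up from zero toward full strength rather than fading out.
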(event `self.ReceiveBeginPlay`
  (`KismetSystemLibrary.Delay` (`self.Lifespan`))
  (`self.K2_DestroyActor`))

(event `self.ReceiveTick`
  (params (DeltaSeconds :type "Float (single-precision)"))
  (set `self.Age` (+ DeltaSeconds (`self.Age`))))

(fn `Get Heat`
  (returns (Heat :type "Float (double-precision)"))
  (return (* (/ (`self.Age`) (`KismetMathLibrary.FMax` (`self.Lifespan`) 0.01)) (`self.Heat`))))

(fn `Get Locomotiveness`
  (returns (Locomotiveness :type "Float (double-precision)"))
  (return (* (/ (`self.Age`) (`KismetMathLibrary.FMax` (`self.Lifespan`) 0.01)) (`self.Locomotive Disturbance`))))

(fn `Get Noisiness`
  (returns (Noisiness :type "Float (double-precision)"))
  (return (* (/ (`self.Age`) (`KismetMathLibrary.FMax` (`self.Lifespan`) 0.01)) (`self.Noisiness`))))

(fn `UserConstructionScript`)