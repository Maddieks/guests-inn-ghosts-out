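; Game instance that holds night and difficulty state and switches the game between main menu and night play.
; Difficulty comes from a non-negative custom value capped at ten, otherwise from the current night's preset, with zero as fallback.
; Both load functions load the same hotel map as a level instance, then set the game mode's started flag and reset it, so that flag distinguishes menu from gameplay.
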(fn `Get Difficulty`
  (returns (Difficulty :type Integer))
  (bind _night_presets (`self.Night Presets`))
  (bind _current_night (`self.Current Night`))
  (if (>= (`self.Custom Difficulty`) 0)
    (return (`KismetMathLibrary.Min` (`self.Custom Difficulty`) 10))
    (elif (and (>= _current_night 0) (< _current_night (`KismetArrayLibrary.Array_Length` _night_presets)))
      (return (`|GetArrayItem` _night_presets _current_night))
      (else
        (return 0)))))

(fn `Load Level`
  (params (Night :type Integer))
  (set `self.Current Night` Night)
  (`LevelStreamingDynamic.LoadLevelInstanceBySoftObjectPtr` "/Game/Levels/HotelMap1.HotelMap1" (0.0 0.0 0.0) (struct) "" null)
  (bind _asbp_gigo_game_mode (cast `/Game/Blueprints/BP_GIGO_GameMode` (`GameplayStatics.GetGameMode`)))
  (set `/Game/Blueprints/BP_GIGO_GameMode.Game Started` true _asbp_gigo_game_mode)
  (`/Game/Blueprints/BP_GIGO_GameMode.Reset` _asbp_gigo_game_mode))

(fn `Load Main Menu`
  (`LevelStreamingDynamic.LoadLevelInstanceBySoftObjectPtr` "/Game/Levels/HotelMap1.HotelMap1" (0.0 0.0 0.0) (struct) "" null)
  (bind _asbp_gigo_game_mode (cast `/Game/Blueprints/BP_GIGO_GameMode` (`GameplayStatics.GetGameMode`)))
  (set `/Game/Blueprints/BP_GIGO_GameMode.Game Started` false _asbp_gigo_game_mode)
  (`/Game/Blueprints/BP_GIGO_GameMode.Reset` _asbp_gigo_game_mode))