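; BP_Computer is an interactable computer that gives BP_JohnGuest access to a security camera menu.
; It creates a WG_SecurityMenu widget at BeginPlay and stores it for later use.
; Interact calls OnBeginGuide on the guest with a position at the Arrow component's tip, the Monitor as look target, and the stored widget.
; Interact returns false for any other interactor.
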(event `self.ReceiveBeginPlay`
  (bind _returnvalue (`|CreateWidget` "/Game/Widgets/WG_SecurityMenu.WG_SecurityMenu_C"))
  (set `self.Cam Menu Widget` _returnvalue))

(fn `Interact`
  (params (Interactor :type "Actor Object Reference"))
  (returns (Success :type Boolean))
  (bind _arrow (`self.Arrow`))
  (bind _asbp_john_guest (cast `/Game/Blueprints/BP_JohnGuest` Interactor)
    (:`then`
      (`/Game/Blueprints/BP_JohnGuest.On Begin Guide` _asbp_john_guest (+ (`SceneComponent.K2_GetComponentLocation` _arrow) (* (`SceneComponent.GetForwardVector` _arrow) (`ArrowComponent.ArrowLength` _arrow))) (`SceneComponent.K2_GetComponentLocation` (`self.Monitor`)) 0.25 (`self.Cam Menu Widget`))
      (return true))
    (:`CastFailed`
      (return false))))

(fn `UserConstructionScript`
  (`parent.UserConstructionScript`))