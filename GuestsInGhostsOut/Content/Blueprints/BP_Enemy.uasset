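; Base ghost enemy that claims a hauntable room from the GameMode, moves there, and is defeated by damage or staying roomless too long.
; Tick updates aggro, retries room selection while roomless, and drives visibility: fading in when aggroed, otherwise hidden except in player menu mode.
; Dynamic material instances on the skeleton control opacity.
; Aggro, movement, reactions and sensor readings (heat, noisiness, locomotiveness) are empty or zero stubs, apparently for child classes.
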(event `self.ReceiveBeginPlay`
  (bind _asbp_gigo_game_mode (cast `/Game/Blueprints/BP_GIGO_GameMode` (`GameplayStatics.GetGameMode`)))
  (set `self.Gamemode Ref` _asbp_gigo_game_mode)
  (`self.Set Visibility` 0.1))

(event `self.ReceiveTick`
  (params (DeltaSeconds :type "Float (single-precision)"))
  (bind _roomless_time (`self.Roomless Time`))
  (bind _visible_time (`self.Visible Time`))
  (if (`self.Alive`)
    (`self.Determine Aggro`)
    (`|ExecutionSequence`
      (:`then_0`
        (`/Engine/EditorBlueprintResources/StandardMacros.IsValid` (`self.Target Room`)
          (:`Is Not Valid`
            (`self.Select Room`)
            (if (< _roomless_time (`self.Roomless Lifespan`))
              (set `self.Roomless Time` (+ _roomless_time DeltaSeconds))
              (else
                (`self.Defeat`))))))
      (:`then_1`
        (if (`self.Is Aggro`)
          (bind _output_get (set `self.Visible Timer` (`KismetMathLibrary.FClamp` (+ DeltaSeconds (`self.Visible Timer`)) 0.0 _visible_time)))
          (`self.Set Visibility` (/ _output_get _visible_time))
          (else
            (bind _gamemode_ref (`self.Gamemode Ref`)
              (:`then`
                (bind _player_ref (`/Game/Blueprints/BP_GIGO_GameMode.Player Ref` _gamemode_ref)
                  (:`then`
                    (if (`/Game/Blueprints/BP_JohnGuest.Menu Mode` _player_ref)
                      (`self.Set Visibility` 1.0)
                      (else
                        (`self.Set Visibility` 0.0 :!label _label))))
                  (:`else`
                    (goto _label))))
              (:`else`
                (goto _label)))))))))

(event `Destroy After Delay`
  (params (Delay :type "Float (double-precision)"))
  (`KismetSystemLibrary.Delay` Delay)
  (`self.K2_DestroyActor`))

(fn `Alive`
  (returns (Alive :type Boolean))
  (return (> (`self.Health`) 0)))

(fn `Damage`
  (bind _result (`/Engine/EditorBlueprintResources/StandardMacros.DecrementInt` (`self.Health`))
    (:`  `
      (`self.On Damage`)
      (if (<= _result 0)
        (`self.Defeat`)))))

(fn `Defeat`
  (bind _target_room (`self.Target Room`)
    (:`then`
      (`/Game/Blueprints/BP_Room.Remove Haunter` _target_room))
    (:`else`
      _))
  (`self.On Defeat`))

(fn `Determine Aggro`)

(fn `Flash Cam React`)

(fn `Get Heat`
  (returns (Heat :type "Float (double-precision)"))
  (return 0.0))

(fn `Get Locomotiveness`
  (returns (Locomotiveness :type "Float (double-precision)"))
  (return 0.0))

(fn `Get Noisiness`
  (returns (Noisiness :type "Float (double-precision)"))
  (return 0.0))

(fn `Move To Location`
  (params (`Target Location` :type "Vector Structure")))

(fn `On Damage`)

(fn `On Defeat`)

(fn `Select Room`
  (bind _asbp_gigo_game_mode (cast `/Game/Blueprints/BP_GIGO_GameMode` (`GameplayStatics.GetGameMode`)))
  (bind _rooms (`/Game/Blueprints/BP_GIGO_GameMode.Get Hauntable Cluster` _asbp_gigo_game_mode 1 0.0))
  (if (> (`KismetArrayLibrary.Array_Length` _rooms) 0)
    (bind _target_room (`self.Target Room`)
      (:`then`
        (`/Game/Blueprints/BP_Room.Remove Haunter` _target_room))
      (:`else`
        _))
    (bind _output (`|GetArrayItem` _rooms))
    (`/Engine/EditorBlueprintResources/StandardMacros.IsValid` _output
      (:`Is Valid`
        (bind _success (`/Game/Blueprints/BP_Room.Add Haunter` _output))
        (if _success
          (bind _output_get (set `self.Target Room` _output))
          (`KismetSystemLibrary.PrintString` (`/Game/Blueprints/BP_Room.Room Name` _output_get))
          (set `self.Roomless Time` 0.0)
          (if (not (`BlueprintSetLibrary.Set_Contains` (`/Game/Blueprints/BP_Room.Ghost Set` _output_get) self))
            (`self.Move To Location` (`SceneComponent.K2_GetComponentLocation` (`/Game/Blueprints/BP_Room.DefaultSceneRoot` _output_get))))
          (else
            (`self.Set Visibility` 0.0 :!label _label))))
      (:`Is Not Valid`
        (goto _label)))
    (else
      (goto _label))))

(fn `Set Visibility`
  (params (Opacity :type "Float (double-precision)"))
  (for _array_element (`self.Materials`)
    (`MaterialInstanceDynamic.SetScalarParameterValue` _array_element "Opacity" (`KismetMathLibrary.FClamp` Opacity))))

(fn `UserConstructionScript`
  (set `self.Health` (`self.MaxHealth`))
  (set `self.Visible Time` (`KismetMathLibrary.FMax` 0.01 (`self.Visible Time`)))
  (for _array_element (`MeshComponent.GetMaterials` (`self.Ghost Skeleton`))
    (bind _returnvalue (`KismetMaterialLibrary.CreateDynamicMaterialInstance` _array_element))
    (`KismetArrayLibrary.Array_Add` (`self.Materials`) _returnvalue)))