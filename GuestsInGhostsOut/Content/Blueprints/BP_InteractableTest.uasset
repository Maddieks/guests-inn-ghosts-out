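; BP_InteractableTest is a test interactable Blueprint with Interact and Highlight functions.
; Interact prints a message with the object's display name and returns true, without using the Interactor.
; Highlight only toggles a Highlighted flag when the requested state differs, with no visual change in these graphs.
; The event graph holds only disabled placeholder events, and construction just calls the parent script.
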(fn `Highlight`
  (params (Highlight :type Boolean))
  (bind _highlighted (`self.Highlighted`))
  (if (and Highlight (not _highlighted))
    (set `self.Highlighted` true)
    (elif (and (not Highlight) _highlighted)
      (set `self.Highlighted` false))))

(fn `Interact`
  (params (Interactor :type "Actor Object Reference"))
  (returns (Success :type Boolean))
  (`KismetSystemLibrary.PrintString` (`KismetStringLibrary.Concat_StrStr` "Interacted with " (`KismetSystemLibrary.GetDisplayName` self)))
  (return true))

(fn `UserConstructionScript`
  (`parent.UserConstructionScript`))